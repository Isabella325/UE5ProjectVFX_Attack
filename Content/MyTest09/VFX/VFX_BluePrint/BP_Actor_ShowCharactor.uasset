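; BP_Actor_ShowCharactor is a VFX test actor that plays a Niagara effect while raising a Cube component, triggered by the J key.
; BeginPlay enables input from player controller 0; pressing J spawns FX_Blue just above the world origin, stores it, and sets StartMove.
; While StartMove is true, Tick moves the Cube steadily upward in world space, pinning X and Y to zero, with no stop condition.
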(event `self.ReceiveBeginPlay`
  (`self.EnableInput` self (`GameplayStatics.GetPlayerController` 0))
  (set `self.startMove` false))

(event `self.ReceiveTick`
  (params (DeltaSeconds :type "Float (single-precision)"))
  (bind _cube (`self.Cube`))
  (if (`self.startMove`)
    (`SceneComponent.K2_SetWorldLocation` _cube (`KismetMathLibrary.MakeVector` 0.0 0.0 (+ (.z (`SceneComponent.K2_GetComponentLocation` _cube)) (* DeltaSeconds 65.0))) false false)))

(event `Key|J`
  (params (Key :type "Key Structure"))
  (:`Pressed`
    (bind _returnvalue (`NiagaraFunctionLibrary.SpawnSystemAtLocation` "/Game/MyTest09/VFX/FX_Blue.FX_Blue" (0.0 0.0 0.1)))
    (set `self.ngSystemObj` _returnvalue)
    (set `self.startMove` true)))

(fn `UserConstructionScript`)